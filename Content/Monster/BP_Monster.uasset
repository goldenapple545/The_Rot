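; Monster character with two separately spawned eyes that follow the player's camera, plus patrol, speed and attack functions.
; BeginPlay spawns BP_Eye actors and snaps them to the mesh's eye sockets; Tick smoothly interpolates each toward the camera.
; Attack plays a montage and calls OnAttackEnd whether it completes or is interrupted.
; GetPatrolRoute exposes the assigned route, and SetMovementSpeed maps idle, walking and running states to max walk speed.
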(event Custom|AttachLEye
  (bind _returnvalue (Game|SpawnActorfromClass "/Game/Monster/BP_Eye.BP_Eye_C" (Transformation|GetActorTransform) "Undefined" "MultiplyWithRoot" 0 0))
  (bind _output_get (Variables|Default|SetLEyeActor _returnvalue))
  (Transformation|AttachComponentToComponent _output_get (Variables|Character|GetMesh) "L_Eye" "SnapToTarget" "SnapToTarget" "SnapToTarget" true))

(event Custom|Attack
  (Animation|Montage|PlayMontage (Variables|Character|GetMesh) "/Game/Whisper/Animations/Montage_Attack.Montage_Attack"
    (:OnCompleted
      _)
    (:OnInterrupted
      _))
  (Default|CallOnAttackEnd))

(event Custom|AttachREye
  (bind _returnvalue (Game|SpawnActorfromClass "/Game/Monster/BP_Eye.BP_Eye_C" (Transformation|GetActorTransform) "Undefined" "MultiplyWithRoot" 0 0))
  (bind _output_get (Variables|Default|SetREyeActor _returnvalue))
  (Transformation|AttachComponentToComponent _output_get (Variables|Character|GetMesh) "R_Eye" "SnapToTarget" "SnapToTarget" "SnapToTarget" true))

(event EventTick
  (params (DeltaSeconds :type Float%20%28single-precision%29))
  (CallFunction|UpdateEyeRotation (Variables|Default|GetREyeActor))
  (CallFunction|UpdateEyeRotation (Variables|Default|GetLEyeActor)))

(event EventBeginPlay
  (CallFunction|AttachREye)
  (CallFunction|AttachLEye))

(fn ConstructionScript
  (|CallParentFunction))

(fn UpdateEyeRotation
  (params (EyeActor :type BP%20Eye%20Object%20Reference))
  (Transformation|SetActorRotation EyeActor (Math|Interpolation|RInterpTo (.rotation (Transformation|GetActorTransform EyeActor)) (Math|Rotator|FindLookatRotation (.location (Transformation|GetActorTransform EyeActor)) (Camera|GetCameraLocation (Game|GetPlayerCameraManager 0))) (Utilities|Time|GetWorldDeltaSeconds) 8.0)))

(fn GetPatrolRoute
  (return (Variables|AI|GetPatrolRoute)))

(fn SetMovementSpeed
  (params (Speed :type E_MovementSpeed%20Enum :default "NewEnumerator0"))
  (bind _output_get (Variables|/Script/Engine.CharacterMovementComponent|SetMaxWalkSpeed (Variables|Character|GetCharacterMovement) (Utilities|Select :Index Speed :NewEnumerator0 0.0 :NewEnumerator1 1e+02 :NewEnumerator2 5e+02)))
  (return _output_get))